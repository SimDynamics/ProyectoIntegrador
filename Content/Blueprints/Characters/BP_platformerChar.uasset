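; BP_platformerChar is a 2D platformer character Blueprint that handles the character's defeat sequence.
; DefeadFunc runs once behind an IsDefeaded guard, disabling capsule collision, releasing the movement plane constraint and calling LaunchOnDefeat for an upward and sideways launch.
; It then triggers the JumpDefeaded jump node on the animation instance and raises the sprite's translucent sort priority so it draws in front.
; The event graph and construction script are empty.
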(event EventBeginPlay)

(event Collision|EventActorBeginOverlap
  (params (OtherActor :type Actor%20Object%20Reference)))

(event EventTick
  (params (DeltaSeconds :type Float%20%28single-precision%29)))

(fn ConstructionScript)

(fn LaunchonDefeat
  (Character|LaunchCharacter (+ (* (Math|Vector|VectorUp) (Variables|Default|GetdefeatUpLaunch)) (* (Class|KismetMathLibrary|VectorRight) (Variables|Default|GetdefeatForwardLaunch_0))) true true))

(fn DefeadFunc
  (if (not (Variables|Default|GetIsDefeaded))
    (Variables|Default|SetIsDefeaded true)
    (Collision|SetCollisionEnabled (Variables|Default|GetCapsuleComponent) "NoCollision")
    (Class|MovementComponent|SetPlaneConstraintEnabled (Variables|Character|GetCharacterMovement) false)
    (CallFunction|LaunchonDefeat)
    (Class|PaperZDAnimInstance|JumptoNode (Class|PaperZDCharacter|GetAnimInstance) "JumpDefeaded" "None")
    (Rendering|SetTranslucentSortPriority (Variables|Default|GetSprite) 1000)))