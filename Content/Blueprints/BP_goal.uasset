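; Level goal actor that wins the game when the BP_Medico character touches it with no bacteria left.
; Overlapping Sphere1 counts remaining BP_Bacteria actors and plays a failure sound if any exist.
; Otherwise a DoOnce plays a sound, hides Sphere and shows the Ganaste win widget.
; A chain of delays then makes the character jump in celebration, removes the widget and restarts through GM_platformer.
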(event OnComponentBeginOverlap(Sphere1)
  (params (OverlappedComponent :type Primitive%20Component%20Object%20Reference) (OtherActor :type Actor%20Object%20Reference) (OtherComp :type Primitive%20Component%20Object%20Reference) (OtherBodyIndex :type Integer) (bFromSweep :type Boolean) (SweepResult :type Hit%20Result%20Structure%20%28by%20ref%29))
  (bind _asbp_medico (Utilities|Casting|CastToBP_Medico OtherActor))
  (Variables|Default|SetAs%20BP%20Medico _asbp_medico)
  (bind _outactors (Actor|GetAllActorsOfClass "/Game/Blueprints/Characters/Bacteria/BP_Bacteria.BP_Bacteria_C"))
  (if (== (Utilities|Array|Length _outactors) 0)
    (Utilities|FlowControl|DoOnce false
      (:Completed
        (Audio|PlaySound2D "/Game/Sounds/o_mp3.o_mp3" 1.0 1.0 0.0 0 0)
        (Rendering|SetVisibility (Variables|Default|GetSphere) false false)
        (bind _returnvalue (UserInterface|CreateWidget "/Game/Blueprints/ganaste.ganaste_C" (Game|GetPlayerController 0)))
        (bind _output_get (Variables|Default|SetOutroWidgetRef _returnvalue))
        (UserInterface|Viewport|AddtoViewport _output_get 0)
        (Utilities|FlowControl|Delay 0.5)
        (Character|Jump (Variables|Default|GetAs%20BP%20Medico))
        (Utilities|FlowControl|Delay 1.0)
        (Character|Jump (Variables|Default|GetAs%20BP%20Medico))
        (Utilities|FlowControl|Delay 1.0)
        (Character|Jump (Variables|Default|GetAs%20BP%20Medico))
        (Utilities|FlowControl|Delay 1.0)
        (Utilities|FlowControl|Delay 2.0)
        (Widget|RemovefromParent (Variables|Default|GetOutroWidgetRef))
        (Utilities|FlowControl|Delay 3.0)
        (bind _asgm_platformer (Utilities|Casting|CastToGM_platformer (Game|GetGameMode)))
        (Default|RestartGame _asgm_platformer)))
    (else
      (Audio|PlaySound2D "/Engine/EditorSounds/Notifications/CompileFailed_Cue.CompileFailed_Cue" 1.0 1.0 0.0 0 0))))

(event EventBeginPlay)

(event Collision|EventActorBeginOverlap
  (params (OtherActor :type Actor%20Object%20Reference)))

(event EventTick
  (params (DeltaSeconds :type Float%20%28single-precision%29)))

(fn ConstructionScript)