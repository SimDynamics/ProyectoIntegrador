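; BP_Bacteria is an enemy character that turns around at walls and ledges and can be stunned and killed.
; WallDetector overlaps trigger a 180-degree turn, as does an empty LedgeDetector, checked each Tick on walkable floor.
; ReceiveAttack subtracts health, plays stun animation and sound, and starts a stun timer.
; LettalAtack handles zero health with defeat, sound, camera shake and a destroy flag; DestroyBacteria removes the actor after a delay.
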(event OnComponentBeginOverlap(wallDetector)
  (params (OverlappedComponent :type Primitive%20Component%20Object%20Reference) (OtherActor :type Actor%20Object%20Reference) (OtherComp :type Primitive%20Component%20Object%20Reference) (OtherBodyIndex :type Integer) (bFromSweep :type Boolean) (SweepResult :type Hit%20Result%20Structure%20%28by%20ref%29))
  (CallFunction|RotateChar))

(event EventBeginPlay
  (Variables|Default|SetcurrentHealth (Variables|Default|GetmaxHealth)))

(event Collision|EventActorBeginOverlap
  (params (OtherActor :type Actor%20Object%20Reference)))

(event EventTick
  (params (DeltaSeconds :type Float%20%28single-precision%29))
  (|CallParentFunction DeltaSeconds)
  (CallFunction|CheckLedge))

(event EventDestroyBacteria
  (Utilities|FlowControl|Delay 3.0)
  (Actor|DestroyActor))

(fn ConstructionScript
  (|CallParentFunction))

(fn RotateChar
  (Transformation|SetActorRotation (Math|Rotator|CombineRotators (Transformation|GetActorRotation) "0.000000,180.000000,0.000000")))

(fn CheckLedge
  (if (.bwalkablefloor (Variables|/Script/Engine.CharacterMovementComponent|GetCurrentFloor (Variables|Character|GetCharacterMovement)))
    (if (not (> (Utilities|Array|Length (Collision|GetOverlappingActors (Variables|Default|GetledgeDetector) 0 :!class /Script/Engine.PrimitiveComponent)) 0))
      (CallFunction|RotateChar))))

(fn ReceiveAttack
  (params (damage :type Float%20%28double-precision%29))
  (Variables|Default|SetcurrentHealth (- (Variables|Default|GetcurrentHealth) damage))
  ;[0.15 0.15 0.15 0.5] aturdir enemigos al golpearlos
  (Variables|Default|SetIsStunned true)
  (Class|PaperZDAnimInstance|JumptoNode (Class|PaperZDCharacter|GetAnimInstance) "JumpStunned" "None")
  (Audio|PlaySound2D "/Engine/VREditor/Sounds/UI/Foliage_Placed.Foliage_Placed" 1.0 33.0 0.0 0 0)
  (Utilities|Time|SetTimerbyEvent (EventDispatchers|CreateEvent :!event ClearStun) (Variables|Default|GetstunLength)))

(fn ClearStun
  (Variables|Default|SetIsStunned false))

(fn LettalAtack?
  (if (<= (Variables|Default|GetcurrentHealth) 0.0)
    ;[0.15 0.15 0.15 0.5] matar enemigos al golpearlos 4 veces
    (CallFunction|DefeadFunc)
    (Audio|PlaySound2D "/Engine/VREditor/Sounds/UI/Foliage_Placed.Foliage_Placed" 1.0 0.5 0.0 0 0)
    (Camera|PlayWorldCameraShake "/Game/cameraShake/CS_enemigoAplastado.CS_enemigoAplastado_C" (Transformation|GetActorLocation) 0.0 1e+04 0.0)
    (Variables|Default|SetCanDestroyActor? true)))